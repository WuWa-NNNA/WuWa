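; Character Blueprint for Luno that handles player-driven camera look, movement and jumping.
; Enhanced Input look events feed controller yaw and pitch, with the vertical axis inverted before it is applied.
; Move input is relative to control rotation, using only yaw for forward so pitch does not affect it, and the full rotation for strafing.
; The jump action triggers Jump when started.
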(event `EnhancedInput|/Game/LJB/Input/GameAction/IA_Look`
  (params (ActionValue :type "Vector2D Structure") (ElapsedSeconds :type "Float (double-precision)") (TriggeredSeconds :type "Float (double-precision)") (InputAction :type "InputAction Object Reference" :default "/Game/LJB/Input/GameAction/IA_Look.IA_Look"))
  ; 카메라 회전
  (:`Triggered`
    (`self.AddControllerYawInput` ActionValue_X)
    (`self.AddControllerPitchInput` (* ActionValue_Y -1.0))))

(event `EnhancedInput|/Game/LJB/Input/GameAction/IA_Move`
  (params (ActionValue :type "Vector2D Structure") (ElapsedSeconds :type "Float (double-precision)") (TriggeredSeconds :type "Float (double-precision)") (InputAction :type "InputAction Object Reference" :default "/Game/LJB/Input/GameAction/IA_Move.IA_Move"))
  (bind (_returnvalue_roll _returnvalue_pitch _returnvalue_yaw) (`KismetMathLibrary.BreakRotator` (`self.GetControlRotation`)))
  ; 이동
  (:`Triggered`
    (`self.AddMovementInput` (`KismetMathLibrary.GetRightVector` (`self.GetControlRotation`)) ActionValue_X)
    (`self.AddMovementInput` (`KismetMathLibrary.GetForwardVector` (`KismetMathLibrary.MakeRotator` 0.0 0.0 _returnvalue_yaw)) ActionValue_Y)))

(event `EnhancedInput|/Game/LJB/Input/GameAction/IA_Jump`
  (params (ActionValue :type Boolean) (ElapsedSeconds :type "Float (double-precision)") (TriggeredSeconds :type "Float (double-precision)") (InputAction :type "InputAction Object Reference" :default "/Game/LJB/Input/GameAction/IA_Jump.IA_Jump"))
  ; 점프
  (:`Started`
    (`self.Jump`)))

(fn `UserConstructionScript`)