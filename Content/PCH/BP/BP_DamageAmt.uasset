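; BP_DamageAmt is a short-lived floating damage number actor that displays a damage value through a widget component.
; On BeginPlay it passes its Dmg value to the W_DamageAmount widget, stopping if that cast fails.
; The MoveT timeline then lerps the actor from its spawn location to a fixed world-space offset, upward and slightly diagonal, and destroys it when finished.
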(event `self.ReceiveBeginPlay`
  (bind _asw_damage_amount (cast `/Game/PCH/UI/Blueprint/W_DamageAmount` (`WidgetComponent.GetWidget` (`self.Widget`))))
  (set `/Game/PCH/UI/Blueprint/W_DamageAmount.Dmg` (`self.Dmg`) _asw_damage_amount)
  (bind _output_get (set `self.StartLoc` (`self.K2_GetActorLocation`)))
  (set `self.EndLoc` (+ _output_get (-25.0 -25.0 100.0)))
  (bind (_direction _move_track) (`Timeline|Move T` :!via `PlayFromStart`)
    (:`Update`
      (`self.K2_SetActorLocation` (`KismetMathLibrary.VLerp` (`self.StartLoc`) (`self.EndLoc`) _move_track)))
    (:`Finished`
      (`self.K2_DestroyActor`))))

(fn `UserConstructionScript`)